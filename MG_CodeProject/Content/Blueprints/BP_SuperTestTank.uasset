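; Player-drivable test tank vehicle pawn that moves on two caterpillar tracks through a WheeledVehicleMovementComponentTank.
; Input axes store throttle and left/right turn values, which Tick converts into throttle and per-track steering inputs.
; Turning without throttle feeds the turn value as throttle and counter-rotates the tracks to pivot in place; reversing inverts steering.
; Track movement values drive material parameters that pan the treads and rotate the wheels.
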(event `InputAxis|MoveForward`
  (params (AxisValue :type "Float (single-precision)"))
  ;[1 1 1] Simple Throttle Value
  (set `self.Throttle` AxisValue))

(event `InputAxis|TankTurnLeft`
  (params (AxisValue :type "Float (single-precision)"))
  ;[1 1 1] Simple Left Right Steering
  (set `self.LeftCaterpillar` AxisValue))

(event `InputAxis|TankTurnRight`
  (params (AxisValue :type "Float (single-precision)"))
  ;[1 1 1] Simple Left Right Steering
  (set `self.RightCaterpillar` AxisValue))

(event `self.ReceiveTick`
  (params (DeltaSeconds :type "Float (single-precision)"))
  (`self.Tank Tick Throttle`)
  (`self.Tank Tick Steering`)
  (`self.Tank Tick Materials`))

(fn `Tank Tick Materials`
  (bind _mesh (`self.Mesh`))
  (bind _mesh_2 (`self.Mesh`))
  (`|ExecutionSequence`
    (:`then_0`
      ;[1 0.6654 0.6172] Pan Material At Right Caterpillar and Rotate Right Wheels
      (`MeshComponent.SetScalarParameterValueOnMaterials` _mesh "PanRightY" (`self.RightCaterpillarMaterialMovement`))
      (`MeshComponent.SetScalarParameterValueOnMaterials` _mesh "RotWheelRight" (`self.RightCaterpillarMaterialMovement`)))
    (:`then_1`
      ;[1 0.6654 0.6172] Pan Material At Left Caterpillar and Rotate Left Wheels
      (`MeshComponent.SetScalarParameterValueOnMaterials` _mesh_2 "PanLeftY" (`self.LeftCaterpillarMaterialMovement`))
      (`MeshComponent.SetScalarParameterValueOnMaterials` _mesh_2 "RotWheelLeft" (`self.LeftCaterpillarMaterialMovement`)))))

(fn `Tank Tick Steering`
  (bind _throttle (`self.Throttle`))
  (bind _returnvalue (> _throttle 0.1))
  (bind _returnvalue_2 (< _throttle -0.1))
  (bind _aswheeled_vehicle_movement_component_tank (cast `WheeledVehicleMovementComponentTank` (`self.VehicleMovement`)))
  (if (> (`self.LeftCaterpillar`) 0.0)
    ;[1 1 1] Tank Turn Left
    (if _returnvalue
      (`WheeledVehicleMovementComponentTank.SetSteeringLeftInput` _aswheeled_vehicle_movement_component_tank 1.0)
      (`WheeledVehicleMovementComponentTank.SetSteeringRightInput` _aswheeled_vehicle_movement_component_tank 0.0)
      (elif _returnvalue_2
        (`WheeledVehicleMovementComponentTank.SetSteeringLeftInput` _aswheeled_vehicle_movement_component_tank -1.0) ; Invert Movement On Move Back
        (`WheeledVehicleMovementComponentTank.SetSteeringRightInput` _aswheeled_vehicle_movement_component_tank 0.0) ; Invert Movement On Move Back
        (else
          (`WheeledVehicleMovementComponentTank.SetSteeringLeftInput` _aswheeled_vehicle_movement_component_tank 1.0) ; This Required for Turn In Place
          (`WheeledVehicleMovementComponentTank.SetSteeringRightInput` _aswheeled_vehicle_movement_component_tank -1.0) ; This Required for Turn In Place
        )))
    (elif (> (`self.RightCaterpillar`) 0.0)
      ;[1 1 1] Tank Turn Right
      (if _returnvalue
        (`WheeledVehicleMovementComponentTank.SetSteeringRightInput` _aswheeled_vehicle_movement_component_tank 1.0)
        (`WheeledVehicleMovementComponentTank.SetSteeringLeftInput` _aswheeled_vehicle_movement_component_tank 0.0)
        (elif _returnvalue_2
          (`WheeledVehicleMovementComponentTank.SetSteeringRightInput` _aswheeled_vehicle_movement_component_tank -1.0) ; Invert Movement On Move Back
          (`WheeledVehicleMovementComponentTank.SetSteeringLeftInput` _aswheeled_vehicle_movement_component_tank 0.0) ; Invert Movement On Move Back
          (else
            (`WheeledVehicleMovementComponentTank.SetSteeringLeftInput` _aswheeled_vehicle_movement_component_tank -1.0) ; This Required for Turn In Place
            (`WheeledVehicleMovementComponentTank.SetSteeringRightInput` _aswheeled_vehicle_movement_component_tank 1.0) ; This Required for Turn In Place
          )))
      (else
        ;[1 1 1] Set values to 0 to avoid movement on input release
        (`WheeledVehicleMovementComponentTank.SetSteeringRightInput` _aswheeled_vehicle_movement_component_tank 0.0)
        (`WheeledVehicleMovementComponentTank.SetSteeringLeftInput` _aswheeled_vehicle_movement_component_tank 0.0)))))

(fn `Tank Tick Throttle`
  (bind _throttle (`self.Throttle`))
  (bind _throttle_2 (`self.Throttle`))
  (bind _leftcaterpillar (`self.LeftCaterpillar`))
  (bind _rightcaterpillar (`self.RightCaterpillar`))
  (bind _returnvalue (/ _throttle_2 2.0))
  (bind _returnvalue_2 (/ _leftcaterpillar 2.0))
  (bind _returnvalue_3 (/ _rightcaterpillar 2.0))
  (`self.Tank Tick Materials`)
  (bind _aswheeled_vehicle_movement_component_tank (cast `WheeledVehicleMovementComponentTank` (`self.VehicleMovement`)))
  (if (or (> _throttle 0.1) (< _throttle -0.1))
    ;[1 1 1] Apply throttle for move forward & back
    (`WheeledVehicleMovementComponent.SetThrottleInput` _aswheeled_vehicle_movement_component_tank _throttle_2)
    (set `self.LeftCaterpillarMaterialMovement` _returnvalue)
    (set `self.RightCaterpillarMaterialMovement` _returnvalue)
    (elif (> (`self.LeftCaterpillar`) 0.1)
      ;[1 1 1] Apply throttle equal to left caterpillar throttle(Tank requires throttle to be enabled whle steering)
      (`WheeledVehicleMovementComponent.SetThrottleInput` _aswheeled_vehicle_movement_component_tank _leftcaterpillar)
      (bind _result (`/Engine/EditorBlueprintResources/StandardMacros.NegateFloat` _returnvalue_2)
        (:`  `
          (set `self.RightCaterpillarMaterialMovement` _result)
          (set `self.LeftCaterpillarMaterialMovement` _returnvalue_2)))
      (elif (> (`self.RightCaterpillar`) 0.1)
        ;[1 1 1] Apply throttle equal to right caterpillar throttle(Tank requires throttle to be enabled whle steering)
        (`WheeledVehicleMovementComponent.SetThrottleInput` _aswheeled_vehicle_movement_component_tank _rightcaterpillar)
        (bind _result_2 (`/Engine/EditorBlueprintResources/StandardMacros.NegateFloat` _returnvalue_3)
          (:`  `
            (set `self.LeftCaterpillarMaterialMovement` _result_2)
            (set `self.RightCaterpillarMaterialMovement` _returnvalue_3)))
        (else
          ;[1 1 1] Set throttle value to 0 if input buttons are not pressed
          (`WheeledVehicleMovementComponent.SetThrottleInput` _aswheeled_vehicle_movement_component_tank 0.0)
          (if (<= (`WheeledVehicleMovementComponent.GetForwardSpeed` _aswheeled_vehicle_movement_component_tank) 350.0)
            (set `self.LeftCaterpillarMaterialMovement` 0.0)
            (set `self.RightCaterpillarMaterialMovement` 0.0)))))))

(fn `UserConstructionScript`)