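; Player-driven tank Blueprint (Thor Mk3) that handles movement input, camera aiming and track animation.
; Move and turn axes send intents to the TankMovement component, while aim axes rotate the azimuth gimbal and spring arm.
; Tick pushes per-side scalar parameters to mesh materials for track panning and wheel rotation.
; Older wheeled-vehicle steering and throttle logic is disconnected, including the only writes to those track values.
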(event `InputAxis|AimAzimuth`
  (params (AxisValue :type "Float (single-precision)"))
  ;[1 1 1] Camera Input Binding
  (`SceneComponent.K2_AddLocalRotation` (`self.Azimuth Gimbal`) (`KismetMathLibrary.MakeRotator` 0.0 0.0 (* AxisValue (`GameplayStatics.GetWorldDeltaSeconds`) 100.0)) false false))

(event `self.ReceiveTick`
  (params (DeltaSeconds :type "Float (single-precision)"))
  (`self.Tank Steering Tick`)
  (`self.Tank Throttle Tick`)
  (`self.Tank Materials Tick`))

(event `InputAction|Fire`
  (params (Key :type "Key Structure" :default "AnyKey"))
  ;[1 1 1] Firing
)

(event `self.ReceiveBeginPlay`
  (`TankMovementComponent.Initialise` (`self.TankMovement`) null null))

(event `InputAxis|MoveForward`
  (params (AxisValue :type "Float (single-precision)"))
  ;[1 1 1] Simple Throttle Value
)

(event `InputAxis|AimElevation`
  (params (AxisValue :type "Float (single-precision)"))
  ;[1 1 1] Camera Input Binding
  (`SceneComponent.K2_AddLocalRotation` (`self.SpringArm`) (`KismetMathLibrary.MakeRotator` 0.0 (* AxisValue (`GameplayStatics.GetWorldDeltaSeconds`) 100.0)) false false))

(event `InputAxis|Move Forward`
  (params (AxisValue :type "Float (single-precision)"))
  ;[1 1 1] Throttle
  (`TankMovementComponent.IntendMoveForward` (`self.TankMovement`) AxisValue))

(event `InputAxis|TankTurnLeft`
  (params (AxisValue :type "Float (single-precision)"))
  ;[1 1 1] Simple Left Right Steering
)

(event `InputAxis|TankTurnRight`
  (params (AxisValue :type "Float (single-precision)"))
  ;[1 1 1] Simple Left Right Steering
)

(event `InputAxis|Turn Right`
  (params (AxisValue :type "Float (single-precision)"))
  ;[1 1 1] Throttle
  (`TankMovementComponent.IntendTurnRight` (`self.TankMovement`) AxisValue))

(fn `Tank Materials Tick`
  (bind _skeletalmesh (`self.SkeletalMesh`))
  (bind _skeletalmesh_2 (`self.SkeletalMesh`))
  (`|ExecutionSequence`
    (:`then_0`
      ;[1 0.6654 0.6172] Pan Material At Right Caterpillar and Rotate Right Wheels
      (`MeshComponent.SetScalarParameterValueOnMaterials` _skeletalmesh "PanRightY" (`self.RightCaterpillarMaterialMovement`))
      (`MeshComponent.SetScalarParameterValueOnMaterials` _skeletalmesh "RotWheelRight" (`self.RightCaterpillarMaterialMovement`)))
    (:`then_1`
      ;[1 0.6654 0.6172] Pan Material At Left Caterpillar and Rotate Left Wheels
      (`MeshComponent.SetScalarParameterValueOnMaterials` _skeletalmesh_2 "PanLeftY" (`self.LeftCaterpillarMaterialMovement`))
      (`MeshComponent.SetScalarParameterValueOnMaterials` _skeletalmesh_2 "RotWheelLeft" (`self.LeftCaterpillarMaterialMovement`)))))

(fn `Tank Steering Tick`)

(fn `Tank Throttle Tick`)

(fn `UserConstructionScript`)