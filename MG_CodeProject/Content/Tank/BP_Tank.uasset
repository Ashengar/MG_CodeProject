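; BP_Tank is a player-controllable tank that handles camera, movement and firing input.
; On BeginPlay it passes the barrel and turret to TankAiming, and both tracks to TankMovement.
; Aim axes rotate an azimuth gimbal for yaw and the SpringArm for pitch, scaled by delta time.
; Throttle and turn axes forward intent to TankMovement, while the Fire action calls Fire.
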(event `self.ReceiveBeginPlay`
  (`TankAimingComponent.Initialise` (`self.TankAiming`) (`self.TankBarrel`) (`self.TankTurret`))
  (`TankMovementComponent.Initialise` (`self.TankMovement`) (`self.TankTrackL`) (`self.TankTrackR`)))

(event `InputAxis|AimAzimuth`
  (params (AxisValue :type "Float (single-precision)"))
  ;[1 1 1] Camera Input Binding
  (`SceneComponent.K2_AddLocalRotation` (`self.Azimuth Gimbal 2`) (`KismetMathLibrary.MakeRotator` 0.0 0.0 (* AxisValue (`GameplayStatics.GetWorldDeltaSeconds`) 100.0)) false false))

(event `InputAction|Fire`
  (params (Key :type "Key Structure" :default "AnyKey"))
  ;[1 1 1] Firing
  (:`Pressed`
    (`self.Fire`)))

(event `InputAxis|AimElevation`
  (params (AxisValue :type "Float (single-precision)"))
  ;[1 1 1] Camera Input Binding
  (`SceneComponent.K2_AddLocalRotation` (`self.SpringArm`) (`KismetMathLibrary.MakeRotator` 0.0 (* AxisValue (`GameplayStatics.GetWorldDeltaSeconds`) 100.0)) false false))

(event `InputAxis|Move Forward`
  (params (AxisValue :type "Float (single-precision)"))
  ;[1 1 1] Throttle
  (`TankMovementComponent.IntendMoveForward` (`self.TankMovement`) AxisValue))

(event `InputAxis|Turn Right`
  (params (AxisValue :type "Float (single-precision)"))
  ;[1 1 1] Throttle
  (`TankMovementComponent.IntendTurnRight` (`self.TankMovement`) AxisValue))

(fn `UserConstructionScript`)