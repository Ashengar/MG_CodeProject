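; Prototype player-driven tank (T80) pawn built on a tank wheeled-vehicle movement component, with gimbal and spring-arm aiming.
; Axis events store throttle and caterpillar values, with turn input also yawing the mesh directly.
; Tick converts these into throttle and left/right steering, covering reversed and in-place turns.
; Track and wheel motion is faked by driving per-side pan and rotation material parameters from the inputs.
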(event `InputAxis|Turn In Place Left`
  (params (AxisValue :type "Float (single-precision)"))
  ;[1 1 1] Turn in place
  (bind _aswheeled_vehicle_movement_component_tank (cast `WheeledVehicleMovementComponentTank` (`self.VehicleMovement`)))
  (`WheeledVehicleMovementComponent.SetThrottleInput` _aswheeled_vehicle_movement_component_tank AxisValue)
  (`WheeledVehicleMovementComponentTank.SetSteeringLeftInput` _aswheeled_vehicle_movement_component_tank 1.0)
  (`WheeledVehicleMovementComponentTank.SetSteeringRightInput` _aswheeled_vehicle_movement_component_tank -1.0))

(event `InputAxis|TankTurnLeft`
  (params (AxisValue :type "Float (single-precision)"))
  (bind _output_get (set `self.RightCaterpillar` AxisValue))
  (bind _output_get_2 (set `self.LeftCaterpillar` _output_get))
  (`SceneComponent.K2_AddRelativeRotation` (`self.Mesh`) (`KismetMathLibrary.MakeRotator` 0.0 0.0 (* _output_get_2 (`self.Turn Speed`))) false false))

(event `InputAxis|TankTurnRight`
  (params (AxisValue :type "Float (single-precision)"))
  ;[1 1 1] Turn Left & Right
)

(event `InputAxis|Turn In Place Right`
  (params (AxisValue :type "Float (single-precision)"))
  ;[1 1 1] Turn in place
)

(event `InputAxis|MoveForward`
  (params (AxisValue :type "Float (single-precision)"))
  ;[1 1 1] Move Forward
  (set `self.Throttle` AxisValue))

(event `InputAxis|AimAzimuth`
  (params (AxisValue :type "Float (single-precision)"))
  ;[1 1 1] Camera Input Binding
  (`SceneComponent.K2_AddLocalRotation` (`self.Gimbal`) (`KismetMathLibrary.MakeRotator` 0.0 0.0 (* AxisValue (`GameplayStatics.GetWorldDeltaSeconds`) 100.0)) false false))

(event `InputAxis|AimElevation`
  (params (AxisValue :type "Float (single-precision)"))
  ;[1 1 1] Camera Input Binding
  (`SceneComponent.K2_AddLocalRotation` (`self.SpringArm1`) (`KismetMathLibrary.MakeRotator` 0.0 (* AxisValue (`GameplayStatics.GetWorldDeltaSeconds`) 100.0)) false false))

(event `self.ReceiveTick`
  (params (DeltaSeconds :type "Float (single-precision)"))
  ;[0.9765 1 0.2171] Tick Movement Input
  (`self.Tank Throttle Tick`)
  (`self.Tank Steering Tick`)
  (`self.Tick Materials`))

(fn `Tank Steering Tick`
  (bind _throttle (`self.Throttle`))
  (bind _returnvalue (> _throttle 0.1))
  (bind _returnvalue_2 (< _throttle -0.1))
  (bind _aswheeled_vehicle_movement_component_tank (cast `WheeledVehicleMovementComponentTank` (`self.VehicleMovement`)))
  (if (> (`self.LeftCaterpillar`) 0.0)
    ;[1 1 1] Tank Turn Left
    (if _returnvalue
      (`WheeledVehicleMovementComponentTank.SetSteeringLeftInput` _aswheeled_vehicle_movement_component_tank 1.0)
      (`WheeledVehicleMovementComponentTank.SetSteeringRightInput` _aswheeled_vehicle_movement_component_tank 0.0)
      (elif _returnvalue_2
        (`WheeledVehicleMovementComponentTank.SetSteeringLeftInput` _aswheeled_vehicle_movement_component_tank -1.0) ; Invert Movement On Move Back
        (`WheeledVehicleMovementComponentTank.SetSteeringRightInput` _aswheeled_vehicle_movement_component_tank 0.0) ; Invert Movement On Move Back
        (else
          (`WheeledVehicleMovementComponentTank.SetSteeringLeftInput` _aswheeled_vehicle_movement_component_tank 1.0) ; This Required for Turn In Place
          (`WheeledVehicleMovementComponentTank.SetSteeringRightInput` _aswheeled_vehicle_movement_component_tank -1.0) ; This Required for Turn In Place
        )))
    (elif (> (`self.RightCaterpillar`) 0.0)
      ;[1 1 1] Tank Turn Right
      (if _returnvalue
        (`WheeledVehicleMovementComponentTank.SetSteeringRightInput` _aswheeled_vehicle_movement_component_tank 1.0)
        (`WheeledVehicleMovementComponentTank.SetSteeringLeftInput` _aswheeled_vehicle_movement_component_tank 0.0)
        (elif _returnvalue_2
          (`WheeledVehicleMovementComponentTank.SetSteeringRightInput` _aswheeled_vehicle_movement_component_tank -1.0) ; Invert Movement On Move Back
          (`WheeledVehicleMovementComponentTank.SetSteeringLeftInput` _aswheeled_vehicle_movement_component_tank 0.0) ; Invert Movement On Move Back
          (else
            (`WheeledVehicleMovementComponentTank.SetSteeringLeftInput` _aswheeled_vehicle_movement_component_tank -1.0) ; This Required for Turn In Place
            (`WheeledVehicleMovementComponentTank.SetSteeringRightInput` _aswheeled_vehicle_movement_component_tank 1.0) ; This Required for Turn In Place
          )))
      (else
        ;[1 1 1] Set values to 0 to avoid movement on input release
        (`WheeledVehicleMovementComponentTank.SetSteeringRightInput` _aswheeled_vehicle_movement_component_tank 0.0)
        (`WheeledVehicleMovementComponentTank.SetSteeringLeftInput` _aswheeled_vehicle_movement_component_tank 0.0)))))

(fn `Tank Throttle Tick`
  (bind _throttle (`self.Throttle`))
  (bind _throttle_2 (`self.Throttle`))
  (bind _leftcaterpillar (`self.LeftCaterpillar`))
  (bind _rightcaterpillar (`self.RightCaterpillar`))
  (bind _returnvalue (/ _rightcaterpillar 2.0))
  (bind _returnvalue_2 (/ _throttle_2 0.5))
  (bind _returnvalue_3 (/ _leftcaterpillar 2.0))
  (bind _aswheeled_vehicle_movement_component_tank (cast `WheeledVehicleMovementComponentTank` (`self.VehicleMovement`)))
  (if (or (> _throttle 0.1) (< _throttle -0.1))
    ;[1 1 1] Apply throttle for move forward & back
    (`WheeledVehicleMovementComponent.SetThrottleInput` _aswheeled_vehicle_movement_component_tank _throttle_2)
    (set `self.LeftCaterpillarMaterialMovement` _returnvalue_2)
    (set `self.RightCaterpillarMaterialMovement` _returnvalue_2)
    (elif (> (`self.LeftCaterpillar`) 0.1)
      ;[1 1 1] Apply throttle equal to left caterpillar throttle(Tank requires throttle to be enabled whle steering)
      (`WheeledVehicleMovementComponent.SetThrottleInput` _aswheeled_vehicle_movement_component_tank _leftcaterpillar)
      (bind _result (`/Engine/EditorBlueprintResources/StandardMacros.NegateFloat` _returnvalue_3)
        (:`  `
          (set `self.RightCaterpillarMaterialMovement` _result)
          (set `self.LeftCaterpillarMaterialMovement` _returnvalue_3)))
      (elif (> (`self.RightCaterpillar`) 0.1)
        ;[1 1 1] Apply throttle equal to right caterpillar throttle(Tank requires throttle to be enabled whle steering)
        (`WheeledVehicleMovementComponent.SetThrottleInput` _aswheeled_vehicle_movement_component_tank _rightcaterpillar)
        (bind _result_2 (`/Engine/EditorBlueprintResources/StandardMacros.NegateFloat` _returnvalue)
          (:`  `
            (set `self.LeftCaterpillarMaterialMovement` _result_2)
            (set `self.RightCaterpillarMaterialMovement` _returnvalue)))
        (else
          ;[1 1 1] Set throttle value to 0 if input buttons are not pressed
          (`WheeledVehicleMovementComponent.SetThrottleInput` _aswheeled_vehicle_movement_component_tank 0.0)
          (if (<= (`WheeledVehicleMovementComponent.GetForwardSpeed` _aswheeled_vehicle_movement_component_tank) 350.0)
            (set `self.LeftCaterpillarMaterialMovement` 0.0)
            (set `self.RightCaterpillarMaterialMovement` 0.0)))))))

(fn `Tick Materials`
  (bind _mesh (`self.Mesh`))
  (bind _mesh_2 (`self.Mesh`))
  (`|ExecutionSequence`
    (:`then_0`
      ;[1 0.6654 0.6172] Pan Material At Right Caterpillar and Rotate Right Wheels
      (`MeshComponent.SetScalarParameterValueOnMaterials` _mesh_2 "PanRightY" (`self.RightCaterpillarMaterialMovement`))
      (`MeshComponent.SetScalarParameterValueOnMaterials` _mesh_2 "RotWheelRight" (`self.RightCaterpillarMaterialMovement`)))
    (:`then_1`
      ;[1 0.6654 0.6172] Pan Material At Left Caterpillar and Rotate Left Wheels
      (`MeshComponent.SetScalarParameterValueOnMaterials` _mesh "PanLeftY" (`self.LeftCaterpillarMaterialMovement`))
      (`MeshComponent.SetScalarParameterValueOnMaterials` _mesh "RotWheelLeft" (`self.LeftCaterpillarMaterialMovement`)))))

(fn `UserConstructionScript`)